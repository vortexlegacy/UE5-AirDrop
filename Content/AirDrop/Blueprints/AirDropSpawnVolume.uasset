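; AirDropSpawnVolume is a placeable volume that periodically spawns AirDrop actors at random navigable locations inside it.
; The construction script caches the sphere component's scaled radius as the spawn radius.
; Tick feeds a Delay of SpawnTime, which paces each spawn at a random navigable point around the sphere's center, relying on nav mesh coverage.
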(event `self.ReceiveTick`
  (params (DeltaSeconds :type "Float (single-precision)"))
  ;[1 1 1] Spawn an "AirDrop". Change the "Spawn Time" variable value to increase or decrease the "AirDrop"s spawn times.
  (`KismetSystemLibrary.Delay` (`self.SpawnTime`))
  (`|SpawnActorFromClass` "/Game/AirDrop/Blueprints/AirDrop.AirDrop_C" (`KismetMathLibrary.MakeTransform` (`NavigationSystemV1.K2_GetRandomLocationInNavigableRadius` (`SceneComponent.K2_GetComponentLocation` (`self.Sphere`)) (`self.Radius`) null null)) "Undefined" "OverrideRootScale" null null))

(fn `UserConstructionScript`
  ;[1 1 1] Set the "AirDrop" scale radious.
  (set `self.Radius` (`SphereComponent.GetScaledSphereRadius` (`self.Sphere`))))