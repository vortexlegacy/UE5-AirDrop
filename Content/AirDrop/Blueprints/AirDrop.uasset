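; Air drop actor: a loot box with a parachute that starts high in the air and descends to the ground.
; BeginPlay lifts the LootBox by a fixed Z offset above its starting location.
; AnyDamage subtracts from Health, and when it equals exactly zero, destroys the Parachute and sets the LootBox's linear damping for a faster fall.
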(event `self.ReceiveBeginPlay`
  (bind _lootbox (`self.LootBox`))
  (bind (_returnvalue_x _returnvalue_y _returnvalue_z) (`KismetMathLibrary.BreakVector` (`SceneComponent.K2_GetComponentLocation` _lootbox)))
  ;[1 1 1] Set the "AirDrop" height location. Change the "float+float" value to increase or decrease the height location.
  (`SceneComponent.K2_SetWorldLocation` _lootbox (`KismetMathLibrary.MakeVector` _returnvalue_x _returnvalue_y (+ _returnvalue_z 8000.0)) false false))

(event `self.ReceiveAnyDamage`
  (params (Damage :type "Float (single-precision)") (DamageType :type "DamageType Object Reference") (InstigatedBy :type "Controller Object Reference") (DamageCauser :type "Actor Object Reference"))
  ;[1 1 1] Set the "AirDrop" health. Once the health is 0 the "Parachute" will destroy itself and the "LootBox" will drop to the ground at a faster speed.
  (bind _output_get (set `self.Health` (- (`self.Health`) Damage)))
  (if (== _output_get 0.0)
    (`ActorComponent.K2_DestroyComponent` (`self.Parachute`))
    (`PrimitiveComponent.SetLinearDamping` (`self.LootBox`) 1.0)))

(fn `UserConstructionScript`)